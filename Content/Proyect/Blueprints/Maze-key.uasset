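; Maze key pickup actor that the player collects by overlapping it.
; On overlap with myCharacter, it briefly sets the character's Tintkey flag, clears it after a short delay, grants the Key flag, then destroys itself.
; Each tick it spins around its Z axis at a speed scaled by the Rotation variable and frame time.
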(event Collision|EventActorBeginOverlap
  (params (OtherActor :type Actor%20Object%20Reference))
  ;[1 1 1] Código para indicar que se ha recogido el item
  (bind _asmy_character (Utilities|Casting|CastTomyCharacter OtherActor))
  (Variables|/Game/Proyect/Blueprints/myCharacter.myCharacter_C|Settintkey _asmy_character true)
  (Utilities|FlowControl|Delay 0.3)
  (Variables|/Game/Proyect/Blueprints/myCharacter.myCharacter_C|Settintkey _asmy_character false)
  (Variables|/Game/Proyect/Blueprints/myCharacter.myCharacter_C|Setkey _asmy_character true)
  (Actor|DestroyActor))

(event EventTick
  (params (DeltaSeconds :type Float%20%28single-precision%29))
  ;[1 1 1] Código para hacer rotar el item en el eje Z
  (Transformation|AddActorLocalRotation (Math|Rotator|MakeRotator 0.0 0.0 (* DeltaSeconds (Variables|Default|Getrotation))) false false))

(fn ConstructionScript)