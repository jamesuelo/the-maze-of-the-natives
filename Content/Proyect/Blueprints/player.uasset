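; Player input Blueprint that drives the myCharacter pawn, cached on BeginPlay: movement, look, jump, lantern toggle and pause.
; Left Shift toggles between walk and run speeds, and pause swaps the HUD and pause widgets.
; Movement axes share a velocity check that, while running without vertical motion, starts a DoOnce-guarded looping timer for footsteps.
; Each step plays a sound and reports a noise event, otherwise the timer is cleared.
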(event Custom|Steps
  (bind _as_my_character (Variables|Default|GetAs%20My%20Character))
  (bind _returnvalue (Transformation|GetActorLocation _as_my_character))
  (Audio|PlaySoundatLocation "/Game/Proyect/Sounds/steps.steps" _returnvalue "0, 0, 0" 1.0 1.0 0.0 0 0 0)
  (Class|AISenseHearing|ReportNoiseEvent _returnvalue 1.0 (Variables|Default|GetAs%20My%20Character) 1e+03 "None"))

(event EventBeginPlay
  ;[1 1 1] Acción para el uso de linterna e inicializar el personaje
  (bind _asmy_character (Utilities|Casting|CastTomyCharacter (Game|GetPlayerCharacter 0)))
  (Variables|Default|SetAs%20My%20Character _asmy_character))

(event Input|ActionEvents|InputActionLantern
  (params (Key :type Key%20Structure :default "None"))
  ;[1 1 1] Acción para el uso de linterna e inicializar el personaje
  (:Pressed
    (Rendering|ToggleVisibility (Variables|/Game/Proyect/Blueprints/myCharacter.myCharacter_C|GetSpotLight (Variables|Default|GetAs%20My%20Character)) false)))

(event Input|ActionEvents|InputActionPauseAction
  (params (Key :type Key%20Structure :default "None"))
  (bind _as_my_character (Variables|Default|GetAs%20My%20Character))
  (bind _reference_pause (Variables|/Game/Proyect/Blueprints/myCharacter.myCharacter_C|Getreference%20pause _as_my_character))
  (bind _refernce_hud (Variables|/Game/Proyect/Blueprints/myCharacter.myCharacter_C|Getrefernce%20HUD _as_my_character))
  ;[1 1 1] Acción para pausar el juego
  (:Pressed
    (if (Game|IsGamePaused)
      (Widget|RemovefromParent _reference_pause)
      (UserInterface|Viewport|AddtoViewport _refernce_hud 0)
      (Game|SetGamePaused false)
      (else
        (Widget|RemovefromParent _refernce_hud)
        (UserInterface|Viewport|AddtoViewport _reference_pause 0)
        (Game|SetGamePaused true)))))

(event Input|ActionEvents|InputActionJumpAction
  (params (Key :type Key%20Structure :default "None"))
  ;[1 1 1] Acciones de salto y movimiento de la cámara
  (:Pressed
    (Character|Jump (Variables|Default|GetAs%20My%20Character))))

(event Input|AxisEvents|InputAxislookRightLeft
  (params (AxisValue :type Float%20%28single-precision%29))
  ;[1 1 1] Acciones de salto y movimiento de la cámara
  (Pawn|Input|AddControllerYawInput (Variables|Default|GetAs%20My%20Character) AxisValue))

(event Input|AxisEvents|InputAxisUD
  (params (AxisValue :type Float%20%28single-precision%29))
  ;[1 1 1] Acciones de salto y movimiento de la cámara
  (Pawn|Input|AddControllerPitchInput (Variables|Default|GetAs%20My%20Character) AxisValue))

(event Input|AxisEvents|InputAxisMove1
  (params (AxisValue :type Float%20%28single-precision%29))
  (bind _as_my_character (Variables|Default|GetAs%20My%20Character))
  (bind _as_my_character_2 (Variables|Default|GetAs%20My%20Character))
  (bind _returnvalue (Transformation|GetVelocity _as_my_character_2))
  ;[1 1 1] Acciones de movimiento del personaje
  (Pawn|Input|AddMovementInput _as_my_character (Math|Vector|GetForwardVector (Pawn|GetControlRotation _as_my_character :!class /Script/Engine.Pawn)) AxisValue false)
  (if (and (and (Math|Boolean|ORBoolean (< (.x _returnvalue) -1.0) (> (.x _returnvalue) 1.0) (< (.y _returnvalue) -1.0) (> (.y _returnvalue) 1.0)) (== (.z _returnvalue) 0.0)) (Variables|/Game/Proyect/Blueprints/myCharacter.myCharacter_C|Getrunning (Variables|Default|GetAs%20My%20Character)))
    (Utilities|FlowControl|DoOnce false :!label _label
      (:Completed
        (bind _returnvalue_2 (Utilities|Time|SetTimerbyEvent (delegate Custom|Steps) 0.4 true))))
    (else
      (Utilities|Time|ClearandInvalidateTimerbyHandle _returnvalue_2)
      (goto _label Reset))))

(event Input|AxisEvents|InputAxisMove2
  (params (AxisValue :type Float%20%28single-precision%29))
  (bind _as_my_character (Variables|Default|GetAs%20My%20Character))
  (bind _as_my_character_2 (Variables|Default|GetAs%20My%20Character))
  (bind _returnvalue (Transformation|GetVelocity _as_my_character_2))
  ;[1 1 1] Acciones de movimiento del personaje
  (Pawn|Input|AddMovementInput _as_my_character (Math|Vector|GetRightVector (Pawn|GetControlRotation _as_my_character :!class /Script/Engine.Pawn)) AxisValue false)
  (if (and (and (Math|Boolean|ORBoolean (< (.x _returnvalue) -1.0) (> (.x _returnvalue) 1.0) (< (.y _returnvalue) -1.0) (> (.y _returnvalue) 1.0)) (== (.z _returnvalue) 0.0)) (Variables|/Game/Proyect/Blueprints/myCharacter.myCharacter_C|Getrunning (Variables|Default|GetAs%20My%20Character)))
    (Utilities|FlowControl|DoOnce false :!label _label
      (:Completed
        (bind _returnvalue_2 (Utilities|Time|SetTimerbyEvent (delegate Custom|Steps) 0.4 true))))
    (else
      (Utilities|Time|ClearandInvalidateTimerbyHandle _returnvalue_2)
      (goto _label Reset))))

(event Input|KeyboardEvents|LeftShift
  (params (Key :type Key%20Structure :default "None"))
  (bind _as_my_character (Variables|Default|GetAs%20My%20Character))
  (bind _as_my_character_2 (Variables|Default|GetAs%20My%20Character))
  (bind _charactermovement (Variables|/Script/Engine.Character|GetCharacterMovement _as_my_character_2))
  ;[1 1 1] Acción para cambiar el movimiento del personaje
  (:Pressed
    (bind _output_get (Variables|/Game/Proyect/Blueprints/myCharacter.myCharacter_C|Setrunning _as_my_character (not (Variables|/Game/Proyect/Blueprints/myCharacter.myCharacter_C|Getrunning _as_my_character))))
    (if _output_get
      (Variables|/Script/Engine.CharacterMovementComponent|SetMaxWalkSpeed _charactermovement 6e+02)
      (else
        (Variables|/Script/Engine.CharacterMovementComponent|SetMaxWalkSpeed _charactermovement 2e+02)))))

(fn ConstructionScript)