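; Door actor that lets the player leave the maze once they hold its key.
; Overlapping the Box checks the character's Key and sets its Alert text, enabling door input only with the key.
; Pressing Use plays the Puerta timeline, which moves the actor by an offset from its location at the press.
; Leaving the Box clears the alert and disables input.
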(event OnComponentBeginOverlap(Box)
  (params (OverlappedComponent :type Primitive%20Component%20Object%20Reference) (OtherActor :type Actor%20Object%20Reference) (OtherComp :type Primitive%20Component%20Object%20Reference) (OtherBodyIndex :type Integer) (bFromSweep :type Boolean) (SweepResult :type Hit%20Result%20Structure%20%28by%20ref%29))
  ;[1 1 1] Código para permitir abrir la puerta en fuuncion de si tiene el item necesario con mensaje de alerta
  (bind _asmy_character (Utilities|Casting|CastTomyCharacter OtherActor))
  (if (Variables|/Game/Proyect/Blueprints/myCharacter.myCharacter_C|Getkey _asmy_character)
    (Variables|/Game/Proyect/Blueprints/myCharacter.myCharacter_C|Setalert _asmy_character "Pulsa E para salir del laberinto")
    (Input|EnableInput (Game|GetPlayerController 0))
    (else
      (Variables|/Game/Proyect/Blueprints/myCharacter.myCharacter_C|Setalert _asmy_character "Debes conseguir primero la llave del laberinto"))))

(event OnComponentEndOverlap(Box)
  (params (OverlappedComponent :type Primitive%20Component%20Object%20Reference) (OtherActor :type Actor%20Object%20Reference) (OtherComp :type Primitive%20Component%20Object%20Reference) (OtherBodyIndex :type Integer))
  ;[1 1 1] Código para permitir abrir la puerta en fuuncion de si tiene el item necesario con mensaje de alerta
  (bind _asmy_character (Utilities|Casting|CastTomyCharacter OtherActor))
  (Variables|/Game/Proyect/Blueprints/myCharacter.myCharacter_C|Setalert _asmy_character "")
  (Input|DisableInput (Game|GetPlayerController 0)))

(event Input|ActionEvents|InputActionUse
  (params (Key :type Key%20Structure))
  ;[1 1 1] Código para abrir la puerta siguiendo un timeline
  (:Pressed
    (bind _output_get (Variables|Default|Setlocation (Transformation|GetActorLocation)))
    (bind _abrir_puerta (Timeline|puerta Play)
      (:Update
        (Transformation|SetActorLocation (+ _output_get _abrir_puerta) false false)))))

(fn ConstructionScript)