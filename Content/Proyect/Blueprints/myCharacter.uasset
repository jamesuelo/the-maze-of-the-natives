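; Player character Blueprint that handles HUD creation, a run/walk toggle and health.
; BeginPlay adds the UI widget to the viewport and creates, but does not display, a Pause widget.
; Left Shift toggles running by switching max walk speed.
; Damage passes through a DoOnce gate that briefly sets a tint flag and ignores further hits until a short delay ends; zero health quits the game.
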(event Custom|c1
  ;[1 1 1] Evento creado para salir del juego
  (Game|QuitGame 0 "Quit" false))

(event EventBeginPlay
  ;[1 1 1] Inicialización para la UI del personaje
  (bind _returnvalue (UserInterface|CreateWidget "/Game/Proyect/Blueprints/UI.UI_C"))
  (bind _output_get (Variables|Default|Setrefernce%20HUD _returnvalue))
  (UserInterface|Viewport|AddtoViewport _output_get 0)
  (bind _returnvalue_2 (UserInterface|CreateWidget "/Game/Proyect/Blueprints/pause.pause_C"))
  (Variables|Default|Setreference%20pause _returnvalue_2))

(event Game|Damage|EventAnyDamage
  (params (Damage :type Float%20%28single-precision%29) (DamageType :type Damage%20Type%20Object%20Reference) (InstigatedBy :type Controller%20Object%20Reference) (DamageCauser :type Actor%20Object%20Reference))
  ;[1 1 1] Aplicación de daño al personaje
  (Utilities|FlowControl|DoOnce false :!label _label
    (:Completed
      (bind _output_get (Variables|Default|SetHealth (- (Variables|Default|GetHealth) Damage)))
      (if (<= _output_get 0.0)
        (CallFunction|C1)
        (else
          (Variables|Default|SettintDamage true)
          (Utilities|FlowControl|Delay 0.2)
          (Variables|Default|SettintDamage false)
          (Utilities|FlowControl|Delay 0.5)
          (goto _label Reset))))))

(event Input|KeyboardEvents|LeftShift
  (params (Key :type Key%20Structure))
  (bind _charactermovement (Variables|Character|GetCharacterMovement))
  ;[1 1 1] Acción para cambiar el movimiento del personaje
  (:Pressed
    (bind _output_get (Variables|Default|Setrunning (not (Variables|Default|Getrunning))))
    (if _output_get
      (Variables|/Script/Engine.CharacterMovementComponent|SetMaxWalkSpeed _charactermovement 6e+02)
      (else
        (Variables|/Script/Engine.CharacterMovementComponent|SetMaxWalkSpeed _charactermovement 2e+02)))))

(fn ConstructionScript)